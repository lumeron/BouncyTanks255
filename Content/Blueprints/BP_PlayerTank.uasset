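; Player tank pawn that aims, fires BP_Bullet2 from its turret, and takes bullet damage.
; Aim axes yaw the whole actor and pitch the spring arm; firing is gated by CanFire.
; A construction-added StatsComponent holds health, which Tick polls to destroy the tank at zero or below and quit if player-controlled.
; Powerup hits are cast, but the health, shield and damage assignment logic is disconnected.
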(event `InputAxis|AimX`
  (params (AxisValue :type "Float (single-precision)"))
  (`self.K2_AddActorWorldRotation` (`KismetMathLibrary.Conv_VectorToRotator` (`KismetMathLibrary.CreateVectorFromYawPitch` (* AxisValue (`self.RotationScale`))))))

(event `InputAxis|AimY`
  (params (AxisValue :type "Float (single-precision)"))
  (`SceneComponent.K2_AddLocalRotation` (`self.springArm`) (`KismetMathLibrary.Conv_VectorToRotator` (`KismetMathLibrary.CreateVectorFromYawPitch` 0.0 (* AxisValue (`self.RotationScale`)))) false false))

(event `InputAction|Fire`
  (params (Key :type "Key Structure"))
  (:`Pressed`
    (if (`self.canFire`)
      (`|SpawnActorFromClass` "/Game/Blueprints/BP_Bullet2.BP_Bullet2_C" (`SceneComponent.K2_GetComponentToWorld` (`self.Turret`)) "Undefined" "OverrideRootScale" (`self.GetOwner`) null))))

(event `self.ReceiveHit`
  (params (MyComp :type "PrimitiveComponent Object Reference") (Other :type "Actor Object Reference") (OtherComp :type "PrimitiveComponent Object Reference") (bSelfMoved :type Boolean) (HitLocation :type "Vector Structure") (HitNormal :type "Vector Structure") (NormalImpulse :type "Vector Structure") (Hit :type "HitResult Structure (by ref)"))
  (bind _returnvalue (`self.GetComponentByClass` "/Script/BouncyTanks255.StatsComponent"))
  (bind _asbp_bullet_2 (cast `/Game/Blueprints/BP_Bullet2` Other)
    (:`then`
      (set `StatsComponent.currentHealth` (- (`StatsComponent.currentHealth` _returnvalue) (`BulletActor.currentDamage` _asbp_bullet_2)) _returnvalue)
      (`self.K2_DestroyActor` _asbp_bullet_2))
    (:`CastFailed`
      (bind _aspowerup_actor (cast `PowerupActor` Other)))))

(event `self.ReceiveTick`
  (params (DeltaSeconds :type "Float (single-precision)"))
  (`/Engine/EditorBlueprintResources/StandardMacros.CompareFloat` (`StatsComponent.currentHealth` (`self.GetComponentByClass` "/Script/BouncyTanks255.StatsComponent"))
    (:`==`
      _)
    (:`<`
      _))
  (`self.K2_DestroyActor`)
  (if (`self.IsPlayerControlled`)
    (`KismetSystemLibrary.QuitGame` null "Quit")))

(fn `UserConstructionScript`
  (`AddComponent|NODE_AddStatsComponent-0`))