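; BP_EnemyTankBase is an enemy tank that shoots at the player, takes damage and collects powerups.
; Player overlap starts a one-second loop spawning BP_Bullet2 from the cannon until overlap ends.
; Bullet hits reduce StatsComponent health; powerup hits raise health, shield or damage and clear the AI controller's state.
; Tick sets that controller to "healing" at low health and destroys the tank at zero or below.
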(event `self.ReceiveHit`
  (params (MyComp :type "PrimitiveComponent Object Reference") (Other :type "Actor Object Reference") (OtherComp :type "PrimitiveComponent Object Reference") (bSelfMoved :type Boolean) (HitLocation :type "Vector Structure") (HitNormal :type "Vector Structure") (NormalImpulse :type "Vector Structure") (Hit :type "HitResult Structure (by ref)"))
  (bind _returnvalue (`self.GetComponentByClass` "/Script/BouncyTanks255.StatsComponent"))
  (bind _asbp_bullet_2 (cast `/Game/Blueprints/BP_Bullet2` Other)
    (:`then`
      (set `StatsComponent.currentHealth` (- (`StatsComponent.currentHealth` _returnvalue) (`BulletActor.currentDamage` _asbp_bullet_2)) _returnvalue)
      (`self.K2_DestroyActor` _asbp_bullet_2))
    (:`CastFailed`
      (bind _aspowerup_actor (cast `PowerupActor` Other))
      (switch `string` (`PowerupActor.powerupGeneratedType` _aspowerup_actor)
        (:`health`
          (bind _powerupgeneratedeffect (`PowerupActor.powerupGeneratedEffect` _aspowerup_actor))
          (set `StatsComponent.currentHealth` (+ (`StatsComponent.currentHealth` _returnvalue) _powerupgeneratedeffect) _returnvalue))
        (:`shield`
          (set `StatsComponent.currentShield` (+ (`StatsComponent.currentShield` _returnvalue) _powerupgeneratedeffect) _returnvalue))
        (:`damage`
          (set `StatsComponent.currentDamage` (+ (`StatsComponent.currentDamage` _returnvalue) _powerupgeneratedeffect) _returnvalue)))
      (bind _asbp_enemy_tank_aicontroller (cast `/Game/Blueprints/AI_EnemyTank/BP_EnemyTankAIController` (`AIBlueprintHelperLibrary.GetAIController` self)))
      (set `EnemyTankAIController.controllerState` "" _asbp_enemy_tank_aicontroller))))

(event `self.ReceiveTick`
  (params (DeltaSeconds :type "Float (single-precision)"))
  (bind _currenthealth (`StatsComponent.currentHealth` (`self.GetComponentByClass` "/Script/BouncyTanks255.StatsComponent")))
  (`/Engine/EditorBlueprintResources/StandardMacros.CompareFloat` _currenthealth 30.0
    (:`>`
      _)
    (:`==`
      _)
    (:`<`
      (bind _asbp_enemy_tank_aicontroller (cast `/Game/Blueprints/AI_EnemyTank/BP_EnemyTankAIController` (`AIBlueprintHelperLibrary.GetAIController` self)))
      (set `EnemyTankAIController.controllerState` "healing" _asbp_enemy_tank_aicontroller)))
  (`/Engine/EditorBlueprintResources/StandardMacros.CompareFloat` _currenthealth
    (:`==`
      _)
    (:`<`
      _))
  (`self.K2_DestroyActor`))

(event `self.ReceiveActorEndOverlap`
  (params (OtherActor :type "Actor Object Reference"))
  (cast `/Game/Blueprints/BP_PlayerTank` OtherActor)
  (set `self.shouldFire` false))

(event `self.ReceiveActorBeginOverlap`
  (params (OtherActor :type "Actor Object Reference"))
  (cast `/Game/Blueprints/BP_PlayerTank` OtherActor)
  (set `self.shouldFire` true)
  (`|SpawnActorFromClass` "/Game/Blueprints/BP_Bullet2.BP_Bullet2_C" (`SceneComponent.K2_GetComponentToWorld` (`self.AICannon`)) "Undefined" "OverrideRootScale" (`self.GetOwner`) null :!label _label)
  (`KismetSystemLibrary.Delay` 1.0)
  (if (`self.shouldFire`)
    (goto _label)))

(fn `UserConstructionScript`)