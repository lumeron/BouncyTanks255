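; Tank-game powerup pickup of type Health, Shield or Damage, with two point lights colored by type in the construction script.
; A hit from BP_Bullet2 (which is destroyed) or BP_PlayerTank hides the powerup and disables its collision.
; It then rerolls after each fixed delay, reappearing on roughly a one-in-five chance.
; No powerup effect is applied in this Blueprint.
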(event `self.ReceiveHit`
  (params (MyComp :type "PrimitiveComponent Object Reference") (Other :type "Actor Object Reference") (OtherComp :type "PrimitiveComponent Object Reference") (bSelfMoved :type Boolean) (HitLocation :type "Vector Structure") (HitNormal :type "Vector Structure") (NormalImpulse :type "Vector Structure") (Hit :type "HitResult Structure (by ref)"))
  (bind _returnvalue (`GameplayStatics.GetObjectClass` Other))
  (if (`self.powerupAvailable`)
    (if (== _returnvalue "/Game/Blueprints/BP_Bullet2.BP_Bullet2_C")
      (`self.K2_DestroyActor` Other) ; destroys bullet instances
      (set `self.powerupAvailable` false :!label _label)
      (`self.SetActorEnableCollision` false)
      (`self.SetActorHiddenInGame` true)
      (if (not (`self.powerupAvailable`)) :!label _label_2
        (`KismetSystemLibrary.Delay` 10.0)
        (if (`KismetMathLibrary.InRange_IntInt` (`KismetMathLibrary.RandomIntegerInRange` 1 100) 40 60)
          (set `self.powerupAvailable` true)
          (`self.SetActorEnableCollision` true)
          (`self.SetActorHiddenInGame` false)
          (else
            (goto _label_2))))
      (elif (== _returnvalue "/Game/Blueprints/BP_PlayerTank.BP_PlayerTank_C")
        (goto _label)))))

(event `self.ReceiveBeginPlay`
  (set `self.powerupAvailable` true)
  (goto _label_2))

(event `self.ReceiveTick`
  (params (DeltaSeconds :type "Float (single-precision)")))

(fn `UserConstructionScript`
  (switch `string` (`|GetEnumeratorNameAsString` (`self.PowerupType`))
    (:`health`
      (`LightComponent.SetLightColor` (`self.PointLight1`) (`KismetMathLibrary.MakeColor` 255.0) true)
      (`LightComponent.SetLightColor` (`self.PointLight2`) (`KismetMathLibrary.MakeColor` 255.0) true))
    (:`shield`
      (`LightComponent.SetLightColor` (`self.PointLight1`) (`KismetMathLibrary.MakeColor` 0.0 0.0 255.0) true)
      (`LightComponent.SetLightColor` (`self.PointLight2`) (`KismetMathLibrary.MakeColor` 0.0 0.0 255.0) true))
    (:`damage`
      (`LightComponent.SetLightColor` (`self.PointLight1`) (`KismetMathLibrary.MakeColor` 0.0 255.0) true)
      (`LightComponent.SetLightColor` (`self.PointLight2`) (`KismetMathLibrary.MakeColor` 0.0 255.0) true))))